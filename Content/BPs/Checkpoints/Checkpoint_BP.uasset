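; Checkpoint actor for a racing game that tracks ordered checkpoint progress, laps and race completion.
; On begin play it caches GameStateBro, then reacts when a SportsCar_Pawn overlaps it.
; Only a checkpoint whose index matches the shared game state counter advances it, enforcing order.
; Reaching the checkpoint maximum resets the counter, then either increments the lap count or calls GameFinished at the lap limit.
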(event EventBeginPlay
  (bind _asgame_state_bro (Utilities|Casting|CastToGameStateBro (Game|GetGameState))
    (:then
      (Variables|Default|Setgamestateref _asgame_state_bro))
    (:CastFailed
      (Development|PrintText "Couldn't get game state"))))

(event Collision|EventActorBeginOverlap
  (params (OtherActor :type Actor%20Object%20Reference))
  (Utilities|Casting|CastToSportsCar_Pawn OtherActor)
  (CallFunction|IncrementCheckpoint)
  (Development|PrintText "Outside Function"))

(event EventTick
  (params (DeltaSeconds :type Float%20%28single-precision%29)))

(fn ConstructionScript)

(fn IncrementCheckpoint
  (bind _gamestateref (Variables|Default|Getgamestateref))
  (Math|Integer|CompareInt (Variables|Default|GetmyIndex) (Variables|/Game/BPs/GameStateBro.GameStateBro_C|GetCheckpoints _gamestateref)
    (:==
      (bind _result (Math|Integer|IncrementInt (Variables|/Game/BPs/GameStateBro.GameStateBro_C|GetCheckpoints _gamestateref))
        (:%20%20
          (bind _output_get (Variables|/Game/BPs/GameStateBro.GameStateBro_C|SetCheckpoints _gamestateref _result))
          (Math|Integer|CompareInt _output_get (Variables|/Game/BPs/GameStateBro.GameStateBro_C|GetMaxCheckPoints _gamestateref)
            (:==
              (Development|PrintText "Lap Finished")
              (Variables|/Game/BPs/GameStateBro.GameStateBro_C|SetCheckpoints _gamestateref 0)
              (Math|Integer|CompareInt (Variables|/Game/BPs/GameStateBro.GameStateBro_C|GetCurrentLapCount _gamestateref) (Variables|/Game/BPs/GameStateBro.GameStateBro_C|GetMaxLaps _gamestateref)
                (:==
                  (Development|PrintText "Game Finished")
                  (Default|GameFinished _gamestateref))
                (:<
                  (bind _result_2 (Math|Integer|IncrementInt (Variables|/Game/BPs/GameStateBro.GameStateBro_C|GetCurrentLapCount _gamestateref))
                    (:%20%20
                      (Variables|/Game/BPs/GameStateBro.GameStateBro_C|SetCurrentLapCount _gamestateref _result_2)
                      (Development|PrintText "Function Finished"))))))))))))